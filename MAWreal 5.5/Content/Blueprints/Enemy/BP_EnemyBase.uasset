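; Base enemy character that delegates health, damage and its own attack tokens to BPCDamageSystem, with an overhead health bar.
; Hit responses play montages and switch AIC_EnemyBase between frozen and attacking; death stops its logic and spawns a corpse.
; Attacks reserve tokens from the target, tracked per target and returned on attack end or death to limit attackers.
; Also exposes team, patrol, range and speed functions, plus an arced-launch jump.
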(event Custom|Die
  (bind _returnvalue (Transformation|GetActorRotation))
  (bind _returnvalue_2 (Transformation|GetActorLocation))
  (Class|BPIGameStateEvents|PublishEnemyDeath(Message) (Game|GetGameState))
  ;[0 0 0 1 30] Die
  (Animation|StopAnimMontage 0)
  (Components|DestroyComponent (Variables|Character|GetMesh))
  (Components|DestroyComponent (Variables|Default|GetHealthBar))
  (Game|SpawnActorfromClass "/Game/Blueprints/InteractionSystem/Interactables/BP_Corpse.BP_Corpse_C" (Math|Transform|MakeTransform (Math|Vector|MakeVector (.x _returnvalue_2) (.y _returnvalue_2) (- (.z _returnvalue_2) 1e+02)) (Math|Rotator|MakeRotator (.roll _returnvalue) (.pitch _returnvalue) (- (.yaw _returnvalue) 45.0)) "1.000000,1.000000,1.000000") "AlwaysSpawn" "MultiplyWithRoot" 0 0)
  (Components|DestroyComponent (Variables|Collision|GetCapsuleComponent))
  (AI|Logic|StopLogic (Variables|/Script/AIModule.AIController|GetBrainComponent (Variables|Default|GetAICEnemyBase)) "")
  (Default|SetStateasDead (Variables|Default|GetAICEnemyBase))
  (bind _keys (Utilities|Map|Keys (Variables|Default|GetReservedAttackTokens)))
  (for _array_element _keys
    (Class|BPIDamageable|ReturnAttackToken(Message) _array_element (.Value (Utilities|Map|Find (Variables|Default|GetReservedAttackTokens) _array_element)))
    (Actor|DestroyActor)))

(event Custom|HitResponse
  (params (OnDamageResponse :type E_DamageResponse%20Enum :default "NewEnumerator0") (DamageCauser :type Actor%20Object%20Reference))
  (bind _hitreactionmontage (Variables|Default|GetHitReactionMontage))
  (bind _staggermontage (Variables|Default|GetStaggerMontage))
  ;[0 0 0 1 30] Hit Response
  (Components|Movement|StopMovementImmediately (Variables|Character|GetCharacterMovement))
  (Default|SetStateasFrozen (Variables|Default|GetAICEnemyBase))
  (Animation|Montage|PlayMontage (Variables|Character|GetMesh) (Utilities|Select :Index OnDamageResponse :NewEnumerator0 _hitreactionmontage :NewEnumerator4 _hitreactionmontage :NewEnumerator5 _hitreactionmontage :NewEnumerator6 (select (Utilities|IsValid _staggermontage) _staggermontage _hitreactionmontage))
    (:OnCompleted
      _)
    (:OnInterrupted
      _))
  (bind _teamnumber (Class|BPIDamageable|GetTeamNumber(Message) DamageCauser))
  (Default|SetStateasAttacking (Variables|Default|GetAICEnemyBase) (select (!= _teamnumber (Variables|Default|GetTeam%20Number)) DamageCauser 0) true))

(event EventJumptoDestination
  (params (Destination :type Vector :default "0, 0, 0"))
  (bind (_x _y _z) (Math|Vector|BreakVector Destination))
  ;[0 0 0 1 30] Jump To Destination
  (bind _outlaunchvelocity (Game|SuggestProjectileVelocityCustomArc (Transformation|GetActorLocation) (Math|Vector|MakeVector _x _y (+ _z 2.5e+02)) 0.0 0.5))
  (Character|LaunchCharacter _outlaunchvelocity true true))

(event EventReturnAttackToken
  (params (AmountReturn :type Integer))
  ;[0 0 0 1 30] Return Attack Token
  (Default|ReturnAttackToken (Variables|Default|GetBPC_DamageSystem) AmountReturn))

(event EventStoreAttackTokens
  (params (AttackTarget :type Actor%20Object%20Reference) (HowMany :type Integer))
  (bind _reservedattacktokens (Variables|Default|GetReservedAttackTokens))
  (bind (_value _returnvalue) (Utilities|Map|Find _reservedattacktokens AttackTarget))
  ;[0 0 0 1 30] Store Attack Tokens
  (Utilities|Map|Add (Variables|Default|GetReservedAttackTokens) AttackTarget (Math|Integer|SelectInt (+ HowMany _value) HowMany _returnvalue)))

(event EventBeginPlay
  (bind _bpc_damagesystem (Variables|Default|GetBPC_DamageSystem))
  ;[0 0 0 1 30] Begin Play
  (bind _returnvalue (UserInterface|CreateWidget "/Game/Blueprints/DamageSystem/W_Healthbar.W_Healthbar_C" 0 self))
  (bind _asaic_enemy_base (Utilities|Casting|CastToAIC_EnemyBase (AI|GetAIController self)))
  (Variables|Default|SetAICEnemyBase _asaic_enemy_base)
  (UserInterface|SetWidget (Variables|Default|GetHealthBar) _returnvalue)
  (Variables|Default|SetHealthBarRef _returnvalue)
  (EventDispatchers|AssignOnDeath _bpc_damagesystem (EventDispatchers|CreateEvent :!event Custom|Die))
  (EventDispatchers|AssignOnDamageResponse _bpc_damagesystem (EventDispatchers|CreateEvent :!event Custom|HitResponse)))

(event EventAttackEnd
  (params (AttackTarget :type Actor%20Object%20Reference))
  ;[0 0 0 1 30] Attack End
  (Utilities|IsValid AttackTarget
    (:Is%20Valid
      (Class|BPIDamageable|ReturnAttackToken(Message) AttackTarget (Variables|Default|GetTokensUsedInCurrentAttack))
      (CallFunction|StoreAttackTokens AttackTarget (* (Variables|Default|GetTokensUsedInCurrentAttack) -1))
      (Variables|Default|SetAttacking false)
      (Default|CallOnAttackEnd))))

(event EventDefaultAttack
  (params (AttackTarget :type Actor%20Object%20Reference))
  ;[0 0 0 1 30] Default Attack
  (Variables|Default|SetAttacking true))

(event EventSetIsInterruptable
  (params (IsInterruptable :type Boolean))
  (Variables|/Game/Blueprints/DamageSystem/BPC_DamageSystem.BPC_DamageSystem_C|SetIsInterruptable (Variables|Default|GetBPC_DamageSystem) IsInterruptable))

(fn ConstructionScript)

(fn AttackStart
  (params (AttackTarget :type Actor%20Object%20Reference) (TokensNeeded :type Integer))
  (bind _success (Class|BPIDamageable|ReserveAttackToken(Message) AttackTarget TokensNeeded))
  (if _success
    (CallFunction|StoreAttackTokens AttackTarget TokensNeeded)
    (Variables|Default|SetTokensUsedInCurrentAttack TokensNeeded)
    (return true)
    (else
      (return false))))

(fn GetCurrentHealth
  (return (Variables|/Game/Blueprints/DamageSystem/BPC_DamageSystem.BPC_DamageSystem_C|GetHealth (Variables|Default|GetBPC_DamageSystem))))

(fn GetIdealRange
  (return 1.5e+02 3.5e+02))

(fn GetIsCloaking
  (return false))

(fn GetMaxHealth
  (return (Variables|/Game/Blueprints/DamageSystem/BPC_DamageSystem.BPC_DamageSystem_C|GetMaxHealth (Variables|Default|GetBPC_DamageSystem))))

(fn GetPatrolRoute
  (return (Variables|AI|GetPatrolRoute)))

(fn GetTeamNumber
  (return (Variables|Default|GetTeam%20Number)))

(fn GetWeaponActor
  (return (Variables|Default|GetWeaponActor)))

(fn Heal
  (params (Amount :type Float%20%28double-precision%29))
  (bind _newhealth (Default|Heal (Variables|Default|GetBPC_DamageSystem) Amount))
  (return _newhealth))

(fn IsAttacking
  (return (Variables|Default|GetAttacking)))

(fn IsDead
  (return (Variables|/Game/Blueprints/DamageSystem/BPC_DamageSystem.BPC_DamageSystem_C|GetIsDead (Variables|Default|GetBPC_DamageSystem))))

(fn ReserveAttackToken
  (params (Amount :type Integer))
  (bind _success (Default|ReserveAttackToken (Variables|Default|GetBPC_DamageSystem) Amount))
  (return _success))

(fn SetMovementSpeed
  (params (MovementSpeed :type E_MovementSpeed%20Enum :default "NewEnumerator0"))
  (bind _output_get (Variables|/Script/Engine.CharacterMovementComponent|SetMaxWalkSpeed (Variables|Character|GetCharacterMovement) (Utilities|Select :Index MovementSpeed :NewEnumerator0 0.0 :NewEnumerator1 1e+02 :NewEnumerator2 3e+02 :NewEnumerator3 5e+02)))
  (return _output_get))

(fn TakeDamage
  (params (DamageInfo :type S%20Damage%20Info%20Structure) (Damage%20Causer :type Actor%20Object%20Reference))
  (bind _wasdamaged (Default|TakeDamage (Variables|Default|GetBPC_DamageSystem) DamageInfo Damage%20Causer))
  (Default|UpdateHealth (Variables|Default|GetHealthBarRef))
  (return _wasdamaged))
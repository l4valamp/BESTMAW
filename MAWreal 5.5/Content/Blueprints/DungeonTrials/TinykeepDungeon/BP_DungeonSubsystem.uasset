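; Dungeon subsystem that procedurally builds a TinyKeep-style layout from seeded random room and corridor classes.
; GenerateDungeon scatters rooms and polls until their physics bodies sleep, with a timeout fallback.
; It then removes overlaps, triangulates a random subset of room centers and turns the MST into L-shaped corridor lines.
; Line traces cull rooms off those lines, scaled corridor actors fill them, and OnDungeonGenerated broadcasts the graph, with optional debug drawing.
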(fn ConstructionScript)

(fn GenerateDungeon
  (params (Seed :type Integer) (RoomClasses :type Array%20of%20BP%20Room%20Base%20Class%20References) (RoomsSpawned :type Integer) (CorridorClasses :type Array%20of%20BP%20Corridor%20Class%20References) (DungeonPosition :type Vector) (DungeonMinBounds :type Vector%202D%20Structure) (DrawBounds :type Boolean) (DrawTriangulation :type Boolean) (DrawMST :type Boolean) (DrawCorridorLines :type Boolean))
  (bind (_x _y) (Math|Vector2D|BreakVector2D DungeonMinBounds))
  (if (or (or (Utilities|Array|IsEmpty RoomClasses) (<= RoomsSpawned 0)) (or (Utilities|Array|IsEmpty CorridorClasses) (or (< _x 0.0) (< _y 0.0))))
    (return false)
    (else
      (Class|KismetMathLibrary|SeedRandomStream (Math|Random|MakeRandomStream Seed))
      (Variables|Default|SetDungeonHeight (.z DungeonPosition))
      (Variables|Default|Setm_CorridorClasses CorridorClasses)
      (Variables|Default|Setm_DrawTriangulation DrawTriangulation)
      (Variables|Default|Setm_DrawMST DrawMST)
      (Variables|Default|Setm_DrawCorridorLines DrawCorridorLines)
      (Variables|Default|Setm_Rooms (CallFunction|CreateRooms RoomClasses RoomsSpawned DungeonPosition DungeonMinBounds))
      (bind _returnvalue (Utilities|Time|SetTimerbyEvent (EventDispatchers|CreateEvent :!event CheckAllRoomsSleeping) 0.05 true))
      (Variables|Default|SetSleepCheckHandle _returnvalue)
      (bind _returnvalue_2 (Utilities|Time|SetTimerbyEvent (EventDispatchers|CreateEvent :!event SafetyCheck) 5.0))
      (LocalVariables|SetSafetyCheckHandle _returnvalue_2)
      (if DrawBounds
        (Rendering|Debug|DrawDebugBox DungeonPosition (Math|Conversions|ToVector(Vector2D) DungeonMinBounds) "(R=1.000000,G=0.000000,B=0.000000,A=1.000000)" "0, 0, 0" 1e+01 1.0)))))

(fn CreateRooms
  (params (RoomClasses :type Array%20of%20BP%20Room%20Base%20Class%20References) (RoomNumber :type Integer) (DungeonPosition :type Vector) (DungeonBounds :type Vector%202D%20Structure))
  (bind (_x _y) (Math|Vector2D|BreakVector2D DungeonBounds))
  (bind (_x_2 _y_2) (Math|Vector2D|BreakVector2D DungeonBounds))
  (Utilities|Array|Shuffle RoomClasses)
  (for _index (range 0 (Math|Integer|Min(Integer) (Utilities|Array|Length RoomClasses) RoomNumber))
    (LocalVariables|SetRotation (Math|Rotator|MakeRotator 0.0 0.0 (.OutItem (Utilities|Array|Random (LocalVariables|GetPossibleAngles)))))
    (bind _returnvalue (Game|SpawnActorfromClass (Utilities|Array|Get(acopy) RoomClasses _index) (Math|Transform|MakeTransform (Math|Vector|MakeVector (+ (.x DungeonPosition) (Math|Random|RandomFloatinRange _x (* _x -1.0))) (+ (.y DungeonPosition) (Math|Random|RandomFloatinRange _y (* _y -1.0))) (.z DungeonPosition)) (LocalVariables|GetRotation) "1.000000,1.000000,1.000000") "Undefined" "MultiplyWithRoot" 0 0))
    (bind _output_get (LocalVariables|SetSpawnedRoom _returnvalue))
    (Utilities|Array|Add (LocalVariables|GetSpawnedRooms) _output_get))
  (for _index_2 (range 0 (- RoomNumber (Utilities|Array|Length RoomClasses)))
    (LocalVariables|SetRotation (Math|Rotator|MakeRotator 0.0 0.0 (.OutItem (Utilities|Array|Random (LocalVariables|GetPossibleAngles)))))
    (bind _returnvalue_2 (Game|SpawnActorfromClass (.OutItem (Utilities|Array|Random RoomClasses)) (Math|Transform|MakeTransform (Math|Vector|MakeVector (+ (.x DungeonPosition) (Math|Random|RandomFloatinRange _x_2 (* _x_2 -1.0))) (+ (.y DungeonPosition) (Math|Random|RandomFloatinRange _y_2 (* _y_2 -1.0))) (.z DungeonPosition)) (LocalVariables|GetRotation) "1.000000,1.000000,1.000000") "Undefined" "MultiplyWithRoot" 0 0))
    (bind _output_get_2 (LocalVariables|SetSpawnedRoom _returnvalue_2))
    (Utilities|Array|Add (LocalVariables|GetSpawnedRooms) _output_get_2))
  (return (LocalVariables|GetSpawnedRooms)))

(fn OnAllRoomsSleep
  (bind _dungeonheight (Variables|Default|GetDungeonHeight))
  (bind _dungeonheight_2 (Variables|Default|GetDungeonHeight))
  (bind _returnvalue (+ _dungeonheight 3e+02))
  (bind _returnvalue_2 (+ _dungeonheight_2 2e+02))
  (CallFunction|RemoveOverlapedRooms (Variables|Default|Getm_Rooms))
  (Development|PrintString (Utilities|String|ToString(Integer) (Utilities|Array|Length (Variables|Default|Getm_Rooms))) true true "(R=0.000000,G=0.660000,B=1.000000,A=1.000000)" 5e+01)
  (bind _outpoints (CallFunction|GetPoints (Variables|Default|Getm_Rooms)))
  (bind _output_get (LocalVariables|SetPoints _outpoints))
  (bind _output_get_2 (LocalVariables|SetTriangles (CallFunction|GenerateTriangulationAlt _output_get)))
  (bind _output_get_3 (LocalVariables|SetMST (.OutLines (CallFunction|GenerateMST _output_get_2))))
  (bind _output_get_4 (LocalVariables|SetCorridorLines (CallFunction|GenerateCorridorLines _output_get_3)))
  (CallFunction|RemoveRoomsNotinCorridorLines (Variables|Default|Getm_Rooms) _output_get_4)
  (LocalVariables|SetM_Corridors (CallFunction|CreateCorridors (LocalVariables|GetCorridorLines)))
  (for _array_element (Variables|Default|Getm_Rooms)
    (Utilities|IsValid _array_element
      (:Is%20Valid
        (Collision|SetActorEnableCollision _array_element false))))
  (Utilities|FlowControl|Sequence
    (:then_0
      (if (Variables|Default|Getm_DrawTriangulation)
        (for _array_element_2 (LocalVariables|GetTriangles)
          (Rendering|Debug|DrawDebugLine (Math|Vector|MakeVector (.X (Math|Vector2D|BreakVector2D (.location (.A (Utilities|Struct|BreakS_Triangle _array_element_2))))) (.Y (Math|Vector2D|BreakVector2D (.location (.A (Utilities|Struct|BreakS_Triangle _array_element_2))))) (+ (Variables|Default|GetDungeonHeight) 1e+02)) (Math|Vector|MakeVector (.X (Math|Vector2D|BreakVector2D (.location (.B (Utilities|Struct|BreakS_Triangle _array_element_2))))) (.Y (Math|Vector2D|BreakVector2D (.location (.B (Utilities|Struct|BreakS_Triangle _array_element_2))))) (+ (Variables|Default|GetDungeonHeight) 1e+02)) "(R=1.000000,G=0.000000,B=0.000000,A=1.000000)" 1e+01 5.0)
          (Rendering|Debug|DrawDebugLine (Math|Vector|MakeVector (.X (Math|Vector2D|BreakVector2D (.location (.B (Utilities|Struct|BreakS_Triangle _array_element_2))))) (.Y (Math|Vector2D|BreakVector2D (.location (.B (Utilities|Struct|BreakS_Triangle _array_element_2))))) (+ (Variables|Default|GetDungeonHeight) 1e+02)) (Math|Vector|MakeVector (.X (Math|Vector2D|BreakVector2D (.location (.C (Utilities|Struct|BreakS_Triangle _array_element_2))))) (.Y (Math|Vector2D|BreakVector2D (.location (.C (Utilities|Struct|BreakS_Triangle _array_element_2))))) (+ (Variables|Default|GetDungeonHeight) 1e+02)) "(R=1.000000,G=0.000000,B=0.000000,A=1.000000)" 1e+01 5.0)
          (Rendering|Debug|DrawDebugLine (Math|Vector|MakeVector (.X (Math|Vector2D|BreakVector2D (.location (.C (Utilities|Struct|BreakS_Triangle _array_element_2))))) (.Y (Math|Vector2D|BreakVector2D (.location (.C (Utilities|Struct|BreakS_Triangle _array_element_2))))) (+ (Variables|Default|GetDungeonHeight) 1e+02)) (Math|Vector|MakeVector (.X (Math|Vector2D|BreakVector2D (.location (.A (Utilities|Struct|BreakS_Triangle _array_element_2))))) (.Y (Math|Vector2D|BreakVector2D (.location (.A (Utilities|Struct|BreakS_Triangle _array_element_2))))) (+ (Variables|Default|GetDungeonHeight) 1e+02)) "(R=1.000000,G=0.000000,B=0.000000,A=1.000000)" 1e+01 5.0))))
    (:then_1
      (if (Variables|Default|Getm_DrawMST)
        (for _array_element_3 (LocalVariables|GetMST)
          (Rendering|Debug|DrawDebugLine (Math|Vector|MakeVector (.X (Math|Vector2D|BreakVector2D (.location (.A (Utilities|Struct|BreakS_Line _array_element_3))))) (.Y (Math|Vector2D|BreakVector2D (.location (.A (Utilities|Struct|BreakS_Line _array_element_3))))) _returnvalue_2) (Math|Vector|MakeVector (.X (Math|Vector2D|BreakVector2D (.location (.B (Utilities|Struct|BreakS_Line _array_element_3))))) (.Y (Math|Vector2D|BreakVector2D (.location (.B (Utilities|Struct|BreakS_Line _array_element_3))))) _returnvalue_2) "(R=0.135348,G=1.000000,B=0.000000,A=1.000000)" 5e+01 2e+01))))
    (:then_2
      (if (Variables|Default|Getm_DrawCorridorLines)
        (for _array_element_4 (LocalVariables|GetCorridorLines)
          (Rendering|Debug|DrawDebugLine (Math|Vector|MakeVector (.X (Math|Vector2D|BreakVector2D (.location (.A (Utilities|Struct|BreakS_Line _array_element_4))))) (.Y (Math|Vector2D|BreakVector2D (.location (.A (Utilities|Struct|BreakS_Line _array_element_4))))) _returnvalue) (Math|Vector|MakeVector (.X (Math|Vector2D|BreakVector2D (.location (.B (Utilities|Struct|BreakS_Line _array_element_4))))) (.Y (Math|Vector2D|BreakVector2D (.location (.B (Utilities|Struct|BreakS_Line _array_element_4))))) _returnvalue) "(R=0.000000,G=0.296772,B=1.000000,A=1.000000)" 0.0 2e+01))))
    (:then_3
      (Utilities|Array|Clear (LocalVariables|GetFinalEdges))
      (for _array_element_5 (LocalVariables|GetMST)
        (Utilities|Array|Add (LocalVariables|GetFinalEdges) (Utilities|Struct|MakeIntPoint (.Index (Utilities|Struct|BreakS_PointwithID (.A (Utilities|Struct|BreakS_Line _array_element_5)))) (.Index (Utilities|Struct|BreakS_PointwithID (.B (Utilities|Struct|BreakS_Line _array_element_5)))))))
      (Default|CallOnDungeonGenerated (.OutPoints (CallFunction|GenerateMST _output_get_2)) (LocalVariables|GetFinalEdges)))))

(fn RemoveOverlapedRooms
  (params (InRooms :type Array%20of%20BP%20Room%20Base%20Object%20References))
  (for _array_element InRooms
    (Utilities|IsValid _array_element
      (:Is%20Valid
        (Physics|SetSimulatePhysics (Variables|/Game/Blueprints/DungeonTrials/GraphGrammarDungeon/Generation/Rooms/BP_RoomBase.BP_RoomBase_C|GetRoomExtent _array_element) false)
        (Collision|SetCollisionProfileName (Variables|/Game/Blueprints/DungeonTrials/GraphGrammarDungeon/Generation/Rooms/BP_RoomBase.BP_RoomBase_C|GetRoomExtent _array_element) "OverlapAll" true :!class /Script/Engine.PrimitiveComponent)
        (bind _output_get (LocalVariables|SetOverlapingActors (Collision|GetOverlappingActors (Variables|/Game/Blueprints/DungeonTrials/GraphGrammarDungeon/Generation/Rooms/BP_RoomBase.BP_RoomBase_C|GetRoomExtent _array_element) "/Game/Blueprints/DungeonTrials/GraphGrammarDungeon/Generation/Rooms/BP_RoomBase.BP_RoomBase_C" :!class /Script/Engine.PrimitiveComponent)))
        (for _array_element_2 _output_get
          (if (!= _array_element_2 _array_element)
            (Utilities|IsValid _array_element_2
              (:Is%20Valid
                (Actor|DestroyActor))))))
      (:Is%20Not%20Valid
        (Utilities|Array|Add (LocalVariables|GetRoomsToRemove) _array_element))))
  (for _array_element_3 (LocalVariables|GetRoomsToRemove)
    (Utilities|Array|RemoveItem (Variables|Default|Getm_Rooms) _array_element_3)))

(fn GetPoints
  (params (InRooms :type Array%20of%20BP%20Room%20Base%20Object%20References))
  (bind _output_get (LocalVariables|SetRoomsCopy InRooms))
  (Utilities|Array|Shuffle _output_get)
  (bind _output_get_2 (LocalVariables|SetNumPointsToGet (Math|Integer|Max(Integer) 4 (/ (Utilities|Array|Length (LocalVariables|GetRoomsCopy)) 4))))
  (LocalVariables|SetNumPointsToGet (Math|Integer|Min(Integer) _output_get_2 (Utilities|Array|Length (LocalVariables|GetRoomsCopy))))
  (for _index (range 0 (LocalVariables|GetNumPointsToGet))
    (Utilities|IsValid (Utilities|Array|Get(acopy) (LocalVariables|GetRoomsCopy) _index)
      (:Is%20Valid
        (Utilities|Array|Add (LocalVariables|GetPoints) (Utilities|Struct|MakeS_PointwithID _index (Math|Vector2D|MakeVector2D (.x (Transformation|GetActorLocation (Utilities|Array|Get(acopy) (LocalVariables|GetRoomsCopy) _index))) (.y (Transformation|GetActorLocation (Utilities|Array|Get(acopy) (LocalVariables|GetRoomsCopy) _index)))))))))
  (return (LocalVariables|GetPoints)))

(fn GenerateCorridorLines
  (params (InMST :type Array%20of%20S%20Line%20Structures))
  (for _array_element InMST
    (LocalVariables|SetIntermediatePoint (select (Math|Random|RandomBool) (Math|Vector2D|MakeVector2D (.X (Math|Vector2D|BreakVector2D (.location (.A (Utilities|Struct|BreakS_Line _array_element))))) (.Y (Math|Vector2D|BreakVector2D (.location (.B (Utilities|Struct|BreakS_Line _array_element)))))) (Math|Vector2D|MakeVector2D (.X (Math|Vector2D|BreakVector2D (.location (.B (Utilities|Struct|BreakS_Line _array_element))))) (.Y (Math|Vector2D|BreakVector2D (.location (.A (Utilities|Struct|BreakS_Line _array_element))))))))
    (Utilities|Array|Add (LocalVariables|GetCorridors) (Utilities|Struct|MakeS_Line (Utilities|Struct|MakeS_PointwithID 0 (.location (.A (Utilities|Struct|BreakS_Line _array_element)))) (Utilities|Struct|MakeS_PointwithID 0 (LocalVariables|GetIntermediatePoint))))
    (Utilities|Array|Add (LocalVariables|GetCorridors) (Utilities|Struct|MakeS_Line (Utilities|Struct|MakeS_PointwithID 0 (LocalVariables|GetIntermediatePoint)) (Utilities|Struct|MakeS_PointwithID 0 (.location (.B (Utilities|Struct|BreakS_Line _array_element)))))))
  (return (LocalVariables|GetCorridors)))

(fn RemoveRoomsNotinCorridorLines
  (params (InRooms :type Array%20of%20BP%20Room%20Base%20Object%20References) (InCorridorLines :type Array%20of%20S%20Line%20Structures))
  (for _array_element InRooms
    (bind _output_get (LocalVariables|SetCurrentRoom _array_element))
    (Collision|SetCollisionProfileName (Variables|/Game/Blueprints/DungeonTrials/GraphGrammarDungeon/Generation/Rooms/BP_RoomBase.BP_RoomBase_C|GetRoomExtent _output_get) "BlockAll" true :!class /Script/Engine.PrimitiveComponent))
  (for _array_element_2 InCorridorLines
    (Utilities|Array|Clear (LocalVariables|GetHits))
    (Utilities|FlowControl|Sequence
      (:then_0
        (bind _outhits (Collision|MultiLineTraceByChannel (Math|Vector|MakeVector (.X (Math|Vector2D|BreakVector2D (.location (.A (Utilities|Struct|BreakS_Line _array_element_2))))) (.Y (Math|Vector2D|BreakVector2D (.location (.A (Utilities|Struct|BreakS_Line _array_element_2))))) (Variables|Default|GetDungeonHeight)) (Math|Vector|MakeVector (.X (Math|Vector2D|BreakVector2D (.location (.B (Utilities|Struct|BreakS_Line _array_element_2))))) (.Y (Math|Vector2D|BreakVector2D (.location (.B (Utilities|Struct|BreakS_Line _array_element_2))))) (Variables|Default|GetDungeonHeight)) "TraceTypeQuery1" false 0 "ForDuration" true "(R=1.000000,G=0.000000,B=0.000000,A=1.000000)" "(R=0.000000,G=1.000000,B=0.000000,A=1.000000)" 5e+01))
        (if (> (Utilities|Array|Length _outhits) 0)
          (for _array_element_3 _outhits
            (bind _asbp_room_base (Utilities|Casting|CastToBP_RoomBase (.HitActor (Collision|BreakHitResult _array_element_3))))
            (if true
              (Utilities|Array|AddUnique (LocalVariables|GetRoomsToKeep) _asbp_room_base)))))
      (:then_1
        (bind _outhits_2 (Collision|MultiLineTraceByChannel (Math|Vector|MakeVector (.X (Math|Vector2D|BreakVector2D (.location (.B (Utilities|Struct|BreakS_Line _array_element_2))))) (.Y (Math|Vector2D|BreakVector2D (.location (.B (Utilities|Struct|BreakS_Line _array_element_2))))) (Variables|Default|GetDungeonHeight)) (Math|Vector|MakeVector (.X (Math|Vector2D|BreakVector2D (.location (.A (Utilities|Struct|BreakS_Line _array_element_2))))) (.Y (Math|Vector2D|BreakVector2D (.location (.A (Utilities|Struct|BreakS_Line _array_element_2))))) (Variables|Default|GetDungeonHeight)) "TraceTypeQuery1" false 0 "ForDuration" true "(R=1.000000,G=0.000000,B=0.000000,A=1.000000)" "(R=0.000000,G=1.000000,B=0.000000,A=1.000000)" 5e+01))
        (if (> (Utilities|Array|Length _outhits_2) 0)
          (for _array_element_4 _outhits_2
            (bind _asbp_room_base_2 (Utilities|Casting|CastToBP_RoomBase (.HitActor (Collision|BreakHitResult _array_element_4))))
            (Utilities|Array|AddUnique (LocalVariables|GetRoomsToKeep) _asbp_room_base_2))))))
  (bind _index (Utilities|ReverseforLoopCustom (- (Utilities|Array|Length (Variables|Default|Getm_Rooms)) 1))
    (:LoopBody
      (bind _output_get_2 (LocalVariables|SetRoomRef (Utilities|Array|Get(acopy) InRooms _index)))
      (Utilities|IsValid _output_get_2
        (:Is%20Valid
          (if (not (Utilities|Array|ContainsItem (LocalVariables|GetRoomsToKeep) (LocalVariables|GetRoomRef)))
            (Actor|DestroyActor (LocalVariables|GetRoomRef))
            (Utilities|Array|RemoveIndex InRooms _index)))))))

(fn CreateCorridors
  (params (InCorridorLines :type Array%20of%20S%20Line%20Structures))
  (for _array_element InCorridorLines
    (LocalVariables|SetCorridorClass (.OutItem (Utilities|Array|Random (Variables|Default|Getm_CorridorClasses))))
    (bind _returnvalue (Game|SpawnActorfromClass (LocalVariables|GetCorridorClass) (Math|Transform|MakeTransform (Math|Vector|MakeVector (.X (Math|Vector2D|BreakVector2D (.location (.A (Utilities|Struct|BreakS_Line _array_element))))) (.Y (Math|Vector2D|BreakVector2D (.location (.A (Utilities|Struct|BreakS_Line _array_element))))) (Variables|Default|GetDungeonHeight)) (Math|Rotator|FindLookatRotation (Math|Conversions|ToVector(Vector2D) (.location (.A (Utilities|Struct|BreakS_Line _array_element)))) (Math|Conversions|ToVector(Vector2D) (.location (.B (Utilities|Struct|BreakS_Line _array_element))))) "1.000000,1.000000,1.000000") "AlwaysSpawn" "MultiplyWithRoot" 0 0))
    (bind _output_get (LocalVariables|SetCorridor _returnvalue))
    (Transformation|SetActorScale3D _output_get (Math|Vector|MakeVector (/ (Math|Vector|Distance(Vector) (Math|Conversions|ToVector(Vector2D) (.location (.A (Utilities|Struct|BreakS_Line _array_element)))) (Math|Conversions|ToVector(Vector2D) (.location (.B (Utilities|Struct|BreakS_Line _array_element))))) 1e+02) 1.0 1.0))
    (Utilities|Array|Add (LocalVariables|GetCorridors) (LocalVariables|GetCorridor)))
  (return (LocalVariables|GetCorridors)))

(fn CheckAllRoomsSleeping
  (bind _array_element (Utilities|Array|ForEachLoopwithBreak (Variables|Default|Getm_Rooms) :!label _label)
    (:LoopBody
      (Utilities|IsValid _array_element
        (:Is%20Valid
          (if (Class|PrimitiveComponent|IsAnyRigidBodyAwake (Variables|/Game/Blueprints/DungeonTrials/GraphGrammarDungeon/Generation/Rooms/BP_RoomBase.BP_RoomBase_C|GetRoomExtent _array_element))
            (LocalVariables|SetAllRoomsSleeping false)
            (goto _label Break)))))
    (:Completed
      (if (and (LocalVariables|GetAllRoomsSleeping) (Utilities|Time|IsValidTimerHandle (Variables|Default|GetSleepCheckHandle)))
        (Utilities|Time|ClearandInvalidateTimerbyHandle (Variables|Default|GetSleepCheckHandle))
        (CallFunction|OnAllRoomsSleep)))))

(fn SafetyCheck
  (if (Utilities|Time|IsValidTimerHandle (Variables|Default|GetSleepCheckHandle))
    (Utilities|Time|ClearandInvalidateTimerbyHandle (Variables|Default|GetSleepCheckHandle))
    (CallFunction|OnAllRoomsSleep)))
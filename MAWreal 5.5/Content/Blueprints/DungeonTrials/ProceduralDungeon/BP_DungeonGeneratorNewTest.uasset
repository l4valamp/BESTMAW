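; Procedural dungeon generator that grows a level from a start room by attaching random rooms at exits, using a seedable random stream.
; Sphere traces screen exits and box overlaps reject colliding rooms, repeating until the room count is reached, then end walls cap open exits.
; A timer check is meant to reload the map if generation stalls.
; Difficulty, door and enemy spawner events exist but their calls are disconnected.
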(event Custom|SpawnStartRoom
  (bind _defaultsceneroot (Variables|Default|GetDefaultSceneRoot))
  (bind _returnvalue (Transformation|GetWorldTransform _defaultsceneroot))
  ;[0 0 0 1 30] Spawn Start Room
  (bind _returnvalue_2 (Game|SpawnActorfromClass :Class "/Game/Blueprints/DungeonTrials/ProceduralDungeon/Rooms/TestNewRooms/BP_TestRoom01.BP_TestRoom01_C" :SpawnTransform _returnvalue :CollisionHandlingOverride "AlwaysSpawn" :TransformScaleMethod "MultiplyWithRoot" :Instigator 0))
  (Utilities|Array|AppendArray (Variables|Default|GetExitsList) (Components|GetChildrenComponents (Variables|/Game/Blueprints/DungeonTrials/ProceduralDungeon/Rooms/BP_MasterRoom.BP_MasterRoom_C|GetExitsFolder _returnvalue_2) false))
  (bind _returnvalue_3 (Game|SpawnActorfromClass "/Game/Blueprints/DungeonTrials/ProceduralDungeon/BP_DistanceBuddy.BP_DistanceBuddy_C" _returnvalue "Undefined" "MultiplyWithRoot" 0 0))
  (Variables|Default|SetDistanceBuddy _returnvalue_3))

(event Custom|TestNextRoom
  ;[0 0 0 1 30] Test Next Room
  (bind _output_get (Variables|Default|SetSelectedExitPoint (.OutItem (Utilities|Array|RandomFromStream (Variables|Default|GetExitsList) (Variables|Default|GetStream)))))
  (bind _returnvalue (Collision|SphereTraceForObjects (+ (.location (Transformation|GetWorldTransform _output_get)) (* (Math|Vector|GetForwardVector _output_get) 5e+02)) (+ (.location (Transformation|GetWorldTransform _output_get)) (* (Math|Vector|GetForwardVector _output_get) 5e+02)) 2e+02 (Utilities|Array|MakeArray "ObjectTypeQuery7") false 0 "None"))
  (if _returnvalue
    (CallFunction|TestNextRoom)
    (else
      (CallFunction|SpawnNextRoom))))

(event Custom|SpawnDoors
  (for _array_element (Variables|Default|GetDoorsList)
    (switch int (Math|Random|RandomIntegerinRange 0 4)
      (:1
        (Game|SpawnActorfromClass (.OutItem (Utilities|Array|RandomFromStream (Variables|Default|GetDoorTypesList) (Variables|Default|GetStream))) (Transformation|GetWorldTransform _array_element) "AlwaysSpawn" "MultiplyWithRoot" 0 0)))))

(event Custom|Spawn%20Next%20Room
  ;[0 0 0 1 30] Spawn Next Room
  (bind _returnvalue (Game|SpawnActorfromClass (.OutItem (Utilities|Array|RandomFromStream (Variables|Default|GetCurrentRoomList) (Variables|Default|GetStream))) (Transformation|GetWorldTransform (Variables|Default|GetSelectedExitPoint)) "AlwaysSpawn" "MultiplyWithRoot" 0 0))
  (bind _asbp_master_room (Utilities|Casting|CastToBP_MasterRoom _returnvalue))
  (Variables|Default|SetLatestRoom _asbp_master_room)
  (Utilities|FlowControl|Delay 0.1) ; This is for fun. Remove for actual game.
  (CallFunction|AddOverlappingRoomstoList)
  (bind _canceltree (CallFunction|CheckOverlappingFunction))
  (if _canceltree
    (Actor|DestroyActor (Variables|Default|GetLatestRoom))
    (CallFunction|TestNextRoom)
    (else
      (Variables|Default|SetRoomAmount (- (Variables|Default|GetRoomAmount) 1))
      (Utilities|Array|RemoveItem (Variables|Default|GetExitsList) (Variables|Default|GetSelectedExitPoint))
      (Utilities|Array|Add (Variables|Default|GetDoorsList) (Variables|Default|GetSelectedExitPoint))
      (Utilities|Array|AppendArray (Variables|Default|GetExitsList) (Components|GetChildrenComponents (Variables|/Game/Blueprints/DungeonTrials/ProceduralDungeon/Rooms/BP_MasterRoom.BP_MasterRoom_C|GetExitsFolder (Variables|Default|GetLatestRoom)) false))
      (Utilities|Array|AppendArray (Variables|Default|GetEnemySpawnList) (Components|GetChildrenComponents (Variables|/Game/Blueprints/DungeonTrials/ProceduralDungeon/Rooms/BP_MasterRoom.BP_MasterRoom_C|GetFloorSpawnPoints (Variables|Default|GetLatestRoom)) false))
      (if (> (Variables|Default|GetRoomAmount) 0) ; If false, runs the events that end the generation process
        ;;[1 1 1] Here's where I would change it to Special Rooms If I Wanted To
        (CallFunction|TestNextRoom)
        (else
          (CallFunction|HandleGaps)
          (CallFunction|CloseEnds)
          (Utilities|Time|ClearandInvalidateTimerbyHandle (Variables|Default|GetTimerHandle))
          (Variables|Default|SetDungeonComplete true))))))

(event Custom|AddOverlappingRoomsToList
  ;[0 0 0 1 30] Check For Overlapping Rooms
  (for _array_element (Components|GetChildrenComponents (Variables|/Game/Blueprints/DungeonTrials/ProceduralDungeon/Rooms/BP_MasterRoom.BP_MasterRoom_C|GetOverlapFolder (Variables|Default|GetLatestRoom)) false)
    (bind _asbox_collision (Utilities|Casting|CastToBoxComponent _array_element))
    (Utilities|Array|AppendArray (Variables|Default|GetOverlappedList) (Class|PrimitiveComponent|GetOverlappingComponents _asbox_collision))))

(event Custom|SelectTargetEnemySpawns
  (bind _stream (Variables|Default|GetStream))
  (bind _enemyspawnlist (Variables|Default|GetEnemySpawnList))
  (bind _outitem (Utilities|Array|RandomFromStream _enemyspawnlist _stream))
  ;[0 0 0 1 30] Random EnemyTarget Spawns
  (if (>= (Variables|Default|GetTargetSpawnAmount) 0) :!label _label
    (bind _output_get (Variables|Default|SetSelectedFloorSpawnLocation _outitem))
    (Transformation|SetActorLocation (Variables|Default|GetDistanceBuddy) (Transformation|GetWorldLocation _output_get) false false)
    (if (and (>= (Math|Vector|Distance(Vector) (Transformation|GetWorldLocation _output_get) (Transformation|GetActorLocation)) (Variables|Default|GetDistanceFromSpawn)) (>= (Class|Actor|GetVerticalDistanceto (Variables|Default|GetDistanceBuddy)) 9e+02))
      (Utilities|Array|Add (Variables|Default|GetTargetEnemySpawnList) _outitem)
      (Utilities|Array|RemoveItem (Variables|Default|GetEnemySpawnList) _outitem)
      (Variables|Default|SetTargetSpawnAmount (- (Variables|Default|GetTargetSpawnAmount) 1))
      (goto _label)
      (else
        (goto _label)))))

(event Custom|SpawnerAtLocation
  ;[0 0 0] Spawn Spawner At Location
  (Variables|Default|SetSpawnerAmount (- (Utilities|Array|Length (Variables|Default|GetEnemySpawnList)) (Variables|Default|GetDungeonDifficulty)))
  (if (>= (Variables|Default|GetSpawnerAmount) 0) :!label _label
    (bind _output_get (Variables|Default|SetSelectedFloorSpawnLocation (.OutItem (Utilities|Array|RandomFromStream (Variables|Default|GetEnemySpawnList) (Variables|Default|GetStream)))))
    (bind _output_get_2 (Variables|Default|SetEnemy%20to%20Spawn (.OutItem (Utilities|Array|RandomFromStream (Variables|Default|GetCurrentEnemyTypesList) (Variables|Default|GetStream)))))
    (Game|SpawnActorfromClass "/Game/Blueprints/DungeonTrials/ProceduralDungeon/Spawns/BP_EnemySpawner.BP_EnemySpawner_C" (Math|Transform|MakeTransform (Transformation|GetWorldLocation _output_get) "0, 0, 0" "1.000000,1.000000,1.000000") "AlwaysSpawn" "MultiplyWithRoot" 0 _output_get_2 false 0)
    (Utilities|Array|RemoveItem (Variables|Default|GetEnemySpawnList) (Variables|Default|GetSelectedFloorSpawnLocation))
    (Development|PrintString (Utilities|String|ToString(Integer) (Utilities|Array|Length (Variables|Default|GetEnemySpawnList))))
    (Variables|Default|SetSpawnerAmount (- (Variables|Default|GetSpawnerAmount) 1))
    (goto _label)))

(event Custom|SpawnDungeon
  ;[0 0 0 1 30] Spawn Dungeon
  (CallFunction|StartDungeonTimer)
  (CallFunction|SpawnStartRoom)
  (CallFunction|TestNextRoom) ; This function starts the looping, first three only run once
)

(event Custom|SetDungeon
  ;[0 0 0 1 30] Set Dungeon Difficulty
  (Variables|Default|SetRoomAmount (+ (* (Variables|Default|GetDungeonDifficulty) 5) 10))
  (Variables|Default|SetTargetSpawnAmount (Variables|Default|GetDungeonDifficulty))
  (Variables|Default|SetSpawnerAmount (- (Variables|Default|GetRoomAmount) (Variables|Default|GetTargetSpawnAmount)))
  (Variables|Default|SetDistanceFromSpawn (Math|Conversions|ToFloat(Integer) (Math|Integer|Clamp(Integer) (+ (* (Variables|Default|GetDungeonDifficulty) 150) 700) 0 1500)))
  (Variables|Default|SetDungeonDifficulty (+ (Variables|Default|GetDungeonDifficulty) 1)))

(event Custom|HandleGaps
  ;[0 0 0 1 30] Handle Gaps
  (for _array_element (Variables|Default|GetExitsList)
    (bind _returnvalue (Collision|SphereTraceForObjects (+ (.location (Transformation|GetWorldTransform _array_element)) (* (Math|Vector|GetForwardVector _array_element) -1e+02)) (+ (.location (Transformation|GetWorldTransform _array_element)) (* (Math|Vector|GetForwardVector _array_element) -1e+02)) 1e+02 (Utilities|Array|MakeArray "ObjectTypeQuery8") false 0 "None"))
    (if (not _returnvalue)
      (Game|SpawnActorfromClass "/Game/Blueprints/DungeonTrials/ProceduralDungeon/Rooms/TestNewRooms/BP_TestEndWall1.BP_TestEndWall1_C" (Transformation|GetWorldTransform _array_element) "AlwaysSpawn" "MultiplyWithRoot" 0 0))))

(event Custom|StartDungeonTimer
  ;[0 0 0 1 30] Dungeon Timer
  (bind _returnvalue (Utilities|Time|SetTimerbyEvent (delegate Custom|CheckForDungeonComplete) 0.0))
  (Variables|Default|SetTimerHandle _returnvalue))

(event Custom|CheckForDungeonComplete
  ;[0 0 0 1 30] Dungeon Timer
  (Development|PrintString "RunningTimer")
  (if (>= (Utilities|Time|GetGameTimeinSeconds) 15.0)
    (Game|OpenLevel(byName) "ThirdPersonMap")))

(event Custom|SetSeed
  ;[0 0 0 1 30] Set Seed
  (if (== (Variables|Default|GetSeed) -1)
    (Class|KismetMathLibrary|SeedRandomStream (Variables|Default|GetStream))
    (else
      (Math|Random|SetRandomStreamSeed (Variables|Default|GetStream) (Variables|Default|GetSeed)))))

(event Custom|SpawnEnemyTargets
  ;[0 0 0 1 30] Spawn Enemy Targets
  (for _array_element (Variables|Default|GetTargetEnemySpawnList)
    (bind _output_get (Variables|Default|SetEnemy%20to%20Spawn (.OutItem (Utilities|Array|RandomFromStream (Variables|Default|GetTargetEnemyTypesList) (Variables|Default|GetStream)))))
    (Game|SpawnActorfromClass "/Game/Blueprints/DungeonTrials/ProceduralDungeon/Spawns/BP_EnemySpawner.BP_EnemySpawner_C" (Math|Transform|MakeTransform (Transformation|GetWorldLocation _array_element) "0, 0, 0" "1.000000,1.000000,1.000000") "AlwaysSpawn" "MultiplyWithRoot" 0 _output_get true 0)))

(event Custom|CloseEnds
  ;[0 0 0 1 30] Close Ends
  (for _array_element (Variables|Default|GetFinalExits)
    (bind _returnvalue (Collision|SphereTraceForObjects (+ (.location (Transformation|GetWorldTransform _array_element)) (* (Math|Vector|GetForwardVector _array_element) -1e+02)) (+ (.location (Transformation|GetWorldTransform _array_element)) (* (Math|Vector|GetForwardVector _array_element) -1e+02)) 1e+02 (Utilities|Array|MakeArray "ObjectTypeQuery8") false 0 "None"))
    (if (not _returnvalue)
      (Game|SpawnActorfromClass :Class "/Game/Blueprints/DungeonTrials/ProceduralDungeon/Rooms/Ends/BP_EndWall.BP_EndWall_C" :SpawnTransform (Transformation|GetWorldTransform _array_element) :CollisionHandlingOverride "Undefined" :TransformScaleMethod "MultiplyWithRoot" :Instigator 0))))

(event EventBeginPlay
  ;[0.5 0 0 1 30] Begin Play
  (CallFunction|SetSeed)
  (CallFunction|SpawnDungeon))

(fn ConstructionScript)

(fn CheckOverlappingFunction
  (CallFunction|AddOverlappingRoomstoList)
  (if (Utilities|Array|IsNotEmpty (Variables|Default|GetOverlappedList))
    (Utilities|Array|Clear (Variables|Default|GetOverlappedList))
    (return true)
    (else
      (Utilities|Array|Clear (Variables|Default|GetOverlappedList))
      (return false))))
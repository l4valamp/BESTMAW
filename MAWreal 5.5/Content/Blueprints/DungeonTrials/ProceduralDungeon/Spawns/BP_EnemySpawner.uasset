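; Enemy spawner for the procedural dungeon that places EnemyToSpawn actors on reachable navmesh points around itself at BeginPlay.
; IsSpawningTarget selects a single spawn in a tight radius; otherwise a random count, possibly zero, spawns over a wider radius.
; SpawnCharacter always spawns despite collision, with a height offset and a yaw from RandomFloat, so only 0–1 degree.
; The node adding spawns to ActivePawns is unconnected, so they are not tracked.
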(event Custom|SpawnInitial
  (for _index (range 1 (Variables|Default|GetSpawnAmount))
    (CallFunction|SpawnCharacter)))

(event EventBeginPlay
  (if (Variables|Default|GetIsSpawningTarget)
    (Variables|Default|SetSpawnAmount 1)
    (Variables|Default|SetRadius 5e+02)
    (else
      (Variables|Default|SetSpawnAmount (Math|Random|RandomInteger 5))
      (Variables|Default|SetRadius 1.5e+03)))
  (CallFunction|SpawnInitial))

(fn ConstructionScript)

(fn SpawnCharacter
  (bind _returnvalue (Transformation|GetActorLocation))
  (bind _radius (Variables|Default|GetRadius))
  (bind _randomlocation (AI|Navigation|GetRandomReachablePointinRadius _returnvalue _radius 0 0))
  (bind _returnvalue_2 (Game|SpawnActorfromClass (Variables|Default|GetEnemyToSpawn) (Math|Transform|MakeTransform (Math|Vector|MakeVector (.x _randomlocation) (.y _randomlocation) (+ (.z _randomlocation) 1e+02)) (Math|Rotator|MakeRotator 0.0 0.0 (Math|Random|RandomFloat)) "1.000000,1.000000,1.000000") "AlwaysSpawn" "MultiplyWithRoot" 0 0)))
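; BP_Door01 is a procedural dungeon door that slides vertically when its Trigger is overlapped.
; Begin and end overlap play separate timelines that lerp StaticMesh from its current relative Z toward raised or lowered targets, without filtering the overlapping actor.
; During each opening update, DoorLights creates new dynamic M_Walls instances on four light components and tints them light blue; closing leaves the tint unchanged.
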(event OnComponentBeginOverlap(Trigger)
  (params (OverlappedComponent :type Primitive%20Component%20Object%20Reference) (OtherActor :type Actor%20Object%20Reference) (OtherComp :type Primitive%20Component%20Object%20Reference) (OtherBodyIndex :type Integer) (bFromSweep :type Boolean) (SweepResult :type Hit%20Result%20Structure%20%28by%20ref%29))
  (bind _staticmesh (Variables|Default|GetStaticMesh))
  (bind _relativelocation (Variables|/Script/Engine.SceneComponent|GetRelativeLocation _staticmesh))
  ;[0 0 0 1 30] Open Door
  (bind _alpha (Timeline|Door%20Animaiton PlayFromStart)
    (:Update
      (Transformation|SetRelativeLocation _staticmesh (Math|Vector|MakeVector (.x _relativelocation) (.y _relativelocation) (Math|Float|Lerp (.z _relativelocation) 9e+02 _alpha)) false false)
      (CallFunction|DoorLights (Variables|Default|GetDoorLight))
      (CallFunction|DoorLights (Variables|Default|GetDoorLight1))
      (CallFunction|DoorLights (Variables|Default|GetDoorLight2))
      (CallFunction|DoorLights (Variables|Default|GetDoorLight3)))))

(event OnComponentEndOverlap(Trigger)
  (params (OverlappedComponent :type Primitive%20Component%20Object%20Reference) (OtherActor :type Actor%20Object%20Reference) (OtherComp :type Primitive%20Component%20Object%20Reference) (OtherBodyIndex :type Integer))
  (bind _staticmesh (Variables|Default|GetStaticMesh))
  (bind _relativelocation (Variables|/Script/Engine.SceneComponent|GetRelativeLocation _staticmesh))
  ;[0 0 0 1 30] Close Door
  (bind _alpha (Timeline|DoorCloseAnimation PlayFromStart)
    (:Update
      (Transformation|SetRelativeLocation _staticmesh (Math|Vector|MakeVector (.x _relativelocation) (.y _relativelocation) (Math|Float|Lerp (.z _relativelocation) -9e+02 _alpha)) false false))))

(event Custom|Door%20Lights
  (params (Light :type Primitive%20Component%20Object%20Reference))
  (bind _returnvalue (Rendering|Material|CreateDynamicMaterialInstance Light 0 "/Game/Blueprints/DungeonTrials/ProceduralDungeon/Materials/M_Walls.M_Walls" "None" :!class /Script/Engine.PrimitiveComponent))
  (Rendering|Material|SetVectorParameterValue _returnvalue "Param" "(R=0.277561,G=0.657893,B=1.000000,A=1.000000)" :!class /Script/Engine.MaterialInstanceDynamic))

(fn ConstructionScript)
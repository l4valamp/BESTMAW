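; BP_DungeonRewriting is an early scaffold for graph-rewriting dungeon generation.
; BeginPlay calls Rewrite, which returns without doing any work; LookForMorphism and VisitMatch are also stubs.
; GenerateMatrix, which nothing here calls, fills the matrix's first row with vertices, debug-prints their index and location, then appends that row once per vertex, leaving edges unprocessed.
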(event EventBeginPlay
  (CallFunction|Rewrite))

(fn ConstructionScript)

(fn GenerateMatrix
  (params (Vertices :type Array%20of%20S%20Pointwith%20ID%20Structures) (Edges :type Array%20of%20S%20Edge%20Structures))
  (LocalVariables|SetLocalVertices Vertices)
  (Variables|Default|SetEdges Edges)
  (for _array_element (LocalVariables|GetLocalVertices)
    (Utilities|Array|Add (Utilities|Struct|BreakS_RowOfNodes (Utilities|Array|Get(acopy) (LocalVariables|GetMatrixStructure))) _array_element)
    (Development|PrintString (Utilities|String|ToString(Text) (Utilities|Text|FormatText "{Index}, ({locationx}, {locationy})" (.Index (Utilities|Struct|BreakS_PointwithID _array_element)) (.x (.Location (Utilities|Struct|BreakS_PointwithID _array_element))) (.y (.Location (Utilities|Struct|BreakS_PointwithID _array_element))))) true true "(R=0.071025,G=0.000000,B=0.156250,A=1.000000)" 1.2e+02))
  (LocalVariables|SetTopNodeRow (Utilities|Array|Get(acopy) (LocalVariables|GetMatrixStructure)))
  (for _array_element_2 (LocalVariables|GetLocalVertices)
    (Utilities|Array|Add (LocalVariables|GetMatrixStructure) (LocalVariables|GetTopNodeRow))))

(fn Rewrite
  (params (RewriteLeft :type Array%20of%20S%20Row%20Of%20Nodes%20Structures) (RewriteRight :type Array%20of%20S%20Row%20Of%20Nodes%20Structures) (BigGraph :type Array%20of%20S%20Row%20Of%20Nodes%20Structures))
  (return 0))

(fn LookforMorphism
  (params (SmallGraph :type Array%20of%20S%20Row%20Of%20Nodes%20Structures) (BigGraph :type Array%20of%20S%20Row%20Of%20Nodes%20Structures)))

(fn VisitMatch
  (return false))
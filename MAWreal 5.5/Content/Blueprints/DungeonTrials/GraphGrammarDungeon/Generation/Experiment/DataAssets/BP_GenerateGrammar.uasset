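; BP_GenerateGrammar is an experimental dungeon generator that expands the DA_Dungeon data asset through a graph grammar on BeginPlay.
; Unfold recursively replaces each non-terminal node with the nodes returned by its ReturnNodeMorphs, appending terminal nodes to GlobalRoomsList.
; CheckifCompleted confirms every collected room is terminal, then BeginPlay prints the flattened room list to screen; no geometry is spawned.
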(event EventBeginPlay
  (bind _iscompleted (CallFunction|Unfold "/Game/Blueprints/DungeonTrials/GraphGrammarDungeon/Generation/Experiment/DataAssets/DA_Dungeon.DA_Dungeon" (Variables|Default|GetGlobalRoomsList)))
  (if _iscompleted
    (for _array_element (Variables|Default|GetGlobalRoomsList)
      (Development|PrintString (Utilities|GetDisplayName _array_element) true true "(R=1.000000,G=0.340547,B=0.000000,A=1.000000)" 6e+01))))

(fn ConstructionScript)

(fn Unfold
  (params (Pick :type Nodes%20Room%201%20Object%20Reference) (RoomsList :type Array%20of%20Nodes%20Room%201%20Object%20References))
  (if (Variables|/Game/Blueprints/DungeonTrials/GraphGrammarDungeon/Generation/Experiment/DataAssets/Nodes_Room1.Nodes_Room1_C|GetTerminal? Pick)
    (Utilities|Array|Add RoomsList Pick)
    (bind _iscompleted (CallFunction|CheckifCompleted))
    (return (Variables|Default|GetGlobalRoomsList) _iscompleted)
    (else
      (Development|PrintString (Utilities|GetDisplayName Pick) true true "(R=0.000000,G=0.134061,B=0.203125,A=1.000000)" 6e+01)
      (bind _roomchosen (Default|ReturnNodeMorphs Pick))
      (for _array_element (Utilities|Struct|BreakS_RoomOptions _roomchosen)
        (CallFunction|Unfold _array_element (Variables|Default|GetGlobalRoomsList)))
      (bind _iscompleted_2 (CallFunction|CheckifCompleted))
      (return (Variables|Default|GetGlobalRoomsList) _iscompleted_2))))

(fn CheckifCompleted
  (LocalVariables|SetCompleted true)
  (for _array_element (Variables|Default|GetGlobalRoomsList)
    (if (not (Variables|/Game/Blueprints/DungeonTrials/GraphGrammarDungeon/Generation/Experiment/DataAssets/Nodes_Room1.Nodes_Room1_C|GetTerminal? _array_element))
      (LocalVariables|SetCompleted false)))
  (return (LocalVariables|GetCompleted)))
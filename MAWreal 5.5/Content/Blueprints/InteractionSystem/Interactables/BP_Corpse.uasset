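; BP_Corpse is an interactable corpse that decays over time and then removes itself.
; On BeginPlay it applies physical animation from a configured bone down and simulates physics only on the bodies below that bone.
; A chain of equal delays moves it through fresh, ripe and rotten flags, swapping materials at the latter two stages before destroying the actor.
; An unconnected full-physics snippet is parked for possible later use.
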(event EventBeginPlay
  (bind _bone (Variables|Default|GetBone))
  ;[1 1 1] Spawn + Rot
  (Class|PhysicalAnimationComponent|SetSkeletalMeshComponent (Variables|Default|GetPhysicalAnimation) (Variables|Default|GetSkeletalMesh))
  (Class|PhysicalAnimationComponent|ApplyPhysicalAnimationSettingsBelow (Variables|Default|GetPhysicalAnimation) _bone (Utilities|Struct|MakePhysicalAnimationData true 1e+03 1e+02 1e+03 1e+03 1e+02 1e+02) true)
  (Class|SkeletalMeshComponent|SetAllBodiesBelowSimulatePhysics (Variables|Default|GetSkeletalMesh) _bone true false)
  (Variables|Default|SetIsFresh true)
  (Utilities|FlowControl|Delay (Variables|Default|GetDelayDuration))
  (Rendering|Material|SetMaterial (Variables|Default|GetSkeletalMesh) 0 "/Game/Blueprints/DungeonTrials/ProceduralDungeon/NewCoolDungeon/MaterialsForTestSquares/M_DungeonBase05.M_DungeonBase05")
  (Variables|Default|SetIsFresh false)
  (Variables|Default|SetIsRipe true)
  (Utilities|FlowControl|Delay (Variables|Default|GetDelayDuration))
  (Rendering|Material|SetMaterial (Variables|Default|GetSkeletalMesh) 0 "/Game/Blueprints/DungeonTrials/ProceduralDungeon/NewCoolDungeon/MaterialsForTestSquares/M_DungeonBase04.M_DungeonBase04")
  (Variables|Default|SetIsRipe false)
  (Variables|Default|SetIsRotten true)
  (Utilities|FlowControl|Delay (Variables|Default|GetDelayDuration))
  (Actor|DestroyActor))

(fn ConstructionScript)
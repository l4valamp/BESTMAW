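; Interactable "Maw" that, when fed, raises dungeon progress and picks the next set of target enemies.
; Feeding sets a placeholder fixed point reward, then randomly draws a progress-scaled number of enemy classes and tallies them into a per-class count map.
; It publishes this state through the GameState on feeding, BeginPlay and dungeon completion.
; Progress and spawn state persist through GameInstance save/load messages, but the chosen targets are not saved.
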(event Custom|DungeonJustCompleted
  (Class|BPIGameStateEvents|PublishMawFed(Message) (Game|GetGameState) 0 (Variables|Default|GetDungeonProgress) (Variables|Default|GetNumberOfTargetEnemies) (Variables|Default|GetChosenTargetEnemies) (Variables|Default|GetEnemyTargets)))

(event Custom|ChooseNewTargetEnemies
  (bind _enemytargets (Variables|Default|GetEnemyTargets))
  (bind _enemytargets_2 (Variables|Default|GetEnemyTargets))
  ;[0 0 0 1 30] On Fed
  ;;[0 0 0 1 30] Choose New Target Enemies
  (Utilities|Map|Clear (Variables|Default|GetEnemyTargets))
  (Utilities|Array|Clear (Variables|Default|GetChosenTargetEnemies))
  (Variables|Default|SetNumberOfTargetEnemies (Math|Random|RandomIntegerinRange (Variables|Default|GetDungeonProgress) (+ (Variables|Default|GetDungeonProgress) 2)))
  (for _index (range 0 (- (Variables|Default|GetNumberOfTargetEnemies) 1))
    (Utilities|Array|Add (Variables|Default|GetChosenTargetEnemies) (.OutItem (Utilities|Array|Random (Variables|Default|GetPotentialTargetEnemies)))))
  (for _array_element (Variables|Default|GetChosenTargetEnemies)
    (if (Utilities|Map|Contains _enemytargets _array_element)
      (Utilities|Map|Add _enemytargets _array_element (+ (.Value (Utilities|Map|Find _enemytargets_2 _array_element)) 1))
      (else
        (Utilities|Map|Add _enemytargets_2 _array_element 1)))))

(event Custom|OnFedCalculations
  (bind _returnvalue (Game|GetGameInstance))
  (bind _asbp_game_instance (Utilities|Casting|CastToBP_GameInstance _returnvalue))
  ;[0 0 0 1 30] On Fed
  (bind _points (CallFunction|CalculatePoints))
  (Variables|Default|SetPointsToGive _points)
  (Variables|Default|SetDungeonProgress (+ (Variables|Default|GetDungeonProgress) 1))
  (CallFunction|ChooseNewTargetEnemies)
  (Class|BPIGameStateEvents|PublishMawFed(Message) (Game|GetGameState) 0 (Variables|Default|GetDungeonProgress) (Variables|Default|GetNumberOfTargetEnemies) (Variables|Default|GetChosenTargetEnemies) (Variables|Default|GetEnemyTargets))
  (CallFunction|SaveData (Variables|/Game/Blueprints/CORE/BP_GameInstance.BP_GameInstance_C|GetSavedGameRef _asbp_game_instance))
  (Class|BPIPersistence|RequestSave(Message) _asbp_game_instance true))

(event EventBeginPlay
  (EventDispatchers|BindEventtoOnDungeonCompleted (.AsGS%20Event%20Manager (Utilities|Casting|CastToGS_EventManager (Game|GetGameState))) (EventDispatchers|CreateEvent :!event Custom|DungeonJustCompleted))
  (Class|BPIPersistence|RequestLoad(Message) (Game|GetGameInstance) self)
  (Class|BPIGameStateEvents|PublishMawFed(Message) (Game|GetGameState) 0 (Variables|Default|GetDungeonProgress) (Variables|Default|GetNumberOfTargetEnemies) (Variables|Default|GetChosenTargetEnemies) (Variables|Default|GetEnemyTargets)))

(event EventInteract
  ;[0 0 0 1 30] Interact
  (CallFunction|OnFedCalculations))

(event EventSaveData
  (params (SavedGameRef :type BP%20Save%20Game%20Object%20Reference))
  (Variables|/Game/Blueprints/CORE/SaveGame/BP_SaveGame.BP_SaveGame_C|SetDungeonResetterSave SavedGameRef (Utilities|Struct|MakeS_DungeonUpgrader (Variables|Default|GetDungeonSpawnable) (Variables|Default|GetDungeonSpawned) (Variables|Default|GetDungeonProgress))))

(event EventLoadData
  (params (SaveGameRef :type BP%20Save%20Game%20Object%20Reference))
  (bind _dungeonresettersave (Variables|/Game/Blueprints/CORE/SaveGame/BP_SaveGame.BP_SaveGame_C|GetDungeonResetterSave SaveGameRef))
  (Variables|Default|SetDungeonSpawned (.dungeonspawned _dungeonresettersave))
  (Variables|Default|SetDungeonSpawnable (.dungeonspawnable _dungeonresettersave))
  (Variables|Default|SetDungeonProgress (.dungeonprogress _dungeonresettersave)))

(fn ConstructionScript)

(fn CalculatePoints
  (return 100))

(fn GetDungeonInfo
  (return ""))
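; Interactable that toggles the dungeon between generation and destruction by publishing messages through the game state.
; Interact requests generation when a dungeon is spawnable, otherwise requests destruction once one is marked as spawned.
; It binds to the GS_EventManager completed and destroyed events, with handler events that set the spawned and spawnable flags.
; The spawned flag is never cleared here.
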(event Custom|MakeDungeonDestructable
  (Variables|Default|SetDungeonSpawned true))

(event Custom|DungeonWasDestroyed
  (Variables|Default|SetDungeonSpawnable true))

(event EventBeginPlay
  (bind _returnvalue (Game|GetGameState))
  (bind _asgs_event_manager (Utilities|Casting|CastToGS_EventManager _returnvalue))
  (EventDispatchers|BindEventtoOnDungeonCompleted _asgs_event_manager (EventDispatchers|CreateEvent :!event Custom|MakeDungeonDestructable))
  (EventDispatchers|BindEventtoOnDungeonDestroyed _asgs_event_manager (EventDispatchers|CreateEvent :!event Custom|DungeonWasDestroyed)))

(event EventInteract
  (bind _returnvalue (Game|GetGameState))
  ;[0 0 0 1 30] Interact
  (if (Variables|Default|GetDungeonSpawnable)
    (Variables|Default|SetDungeonSpawnable false)
    (Class|BPIGameStateEvents|PublishGenerateDungeon(Message) _returnvalue)
    (elif (Variables|Default|GetDungeonSpawned)
      (Class|BPIGameStateEvents|PublishDestroyDungeon(Message) _returnvalue))))

(fn ConstructionScript)

(fn CalculatePoints
  (return 100))

(fn GetDungeonInfo
  (return ""))
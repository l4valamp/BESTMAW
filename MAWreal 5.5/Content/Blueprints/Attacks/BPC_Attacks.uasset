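; Attack component that gives its owning character a library of melee, magic, ranged and AOE attacks, plus an AOE heal.
; Most attacks play a montage whose notifies fire shared projectile, sphere-trace, bullet-trace or spawned-AOE helpers, then message the owner on completion or interruption.
; Trace and generic AOE damage skip teammates by team number.
; The leap launches the character on an arc toward the target's velocity-predicted position.
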(event Custom|DamageEnemyAOE
  (params (Actor :type Actor%20Object%20Reference))
  ;[0 0 0 1 70] AOE
  ;;[0 0 0 1 30] AOE Lightning Strike
  (Class|BPIDamageable|TakeDamage(Message) Actor))

(event Custom|MagicSpell
  (params (SpawnTransform :type Transform) (AttackTarget :type Actor%20Object%20Reference) (DamageInfo :type S%20Damage%20Info%20Structure) (Alt :type Boolean))
  ;[0 0 0 1 70] Misc
  ;;[0 0 0 1 30] Magic Spell
  (bind _returnvalue (Game|SpawnActorfromClass (select Alt "/Game/Blueprints/Attacks/Projectiles/BP_Projectile_DarkEnergy_Alt.BP_Projectile_DarkEnergy_Alt_C" "/Game/Blueprints/Attacks/Projectiles/BP_Projectile_DarkEnergy.BP_Projectile_DarkEnergy_C") SpawnTransform "Undefined" "MultiplyWithRoot" (Components|GetOwner) 1e+03 0.0 AttackTarget false 0))
  (EventDispatchers|AssignOnProjectileImpact _returnvalue (delegate Custom|OnProjectileHit))
  (Collision|IgnoreActorwhenMoving (Actor|GetComponentbyClass (Components|GetOwner) "/Script/Engine.CapsuleComponent") _returnvalue true))

(event Custom|AOEDamageActor
  (params (Actor :type Actor%20Object%20Reference))
  (bind _returnvalue (Components|GetOwner))
  ;[0 0 0 1 70] AOE
  ;;[0 0 0 1 30] AOE Damage
  (bind _teamnumber (Class|BPIDamageable|GetTeamNumber(Message) Actor))
  (bind _teamnumber_2 (Class|BPIDamageable|GetTeamNumber(Message) _returnvalue))
  (if (!= _teamnumber _teamnumber_2)
    (Class|BPIDamageable|TakeDamage(Message) Actor (stale Custom|AOEDamage DamageInfo) _returnvalue)))

(event Custom|FireBullet
  (params (TraceStart :type Vector) (TraceEnd :type Vector) (DamageInfo :type S%20Damage%20Info%20Structure))
  ;[0 0 0 1 70] AOE
  ;;[0 0 0 1 30] Fire Bullet
  (bind (_outhits _returnvalue) (Class|KismetSystemLibrary|LineTraceMultiforObjects TraceStart TraceEnd (Utilities|Array|MakeArray "ObjectTypeQuery3") false (Utilities|Array|MakeArray (Components|GetOwner)) "ForDuration" true))
  (if _returnvalue
    (bind _damagedactor (CallFunction|DamageFirstNonTeamMember _outhits DamageInfo))
    (Class|AISenseDamage|ReportDamageEvent _damagedactor 0 (Utilities|Struct|BreakS_DamageInfo DamageInfo) (Transformation|GetActorLocation (Components|GetOwner)) "0, 0, 0" "None")))

(event Custom|SpinningAttack
  (params (AttackInfo :type S%20Attack%20Info%20Structure) (Radius :type Float%20%28single-precision%29))
  (bind (_attacktarget _montage _damageinfo) (Utilities|Struct|BreakS_AttackInfo AttackInfo))
  (bind _returnvalue (Components|GetOwner))
  ;[0 0 0 1 70] Melee
  ;;[0 0 0 1 30] Spinning Attack
  (bind _mesh (CallFunction|AttackBase _attacktarget))
  (bind _notifyname (Animation|Montage|PlayMontage _mesh _montage)
    (:OnCompleted
      (Class|BPIEnemyAI|AttackEnd(Message) _returnvalue _attacktarget :!label _label)
      (Class|BPIDamageable|SetIsInterruptable(Message) _returnvalue true))
    (:OnInterrupted
      (goto _label))
    (:OnNotifyBegin
      (switch name _notifyname
        (:Slash
          (CallFunction|SphereTraceDamage :Length 2e+01 :Radius Radius))
        (:AOESlash
          (CallFunction|AOEDamage Radius _damageinfo))))))

(event Custom|HealTarget
  (params (HealTarget :type Actor%20Object%20Reference))
  (bind _returnvalue (Transformation|GetActorLocation HealTarget))
  ;[0 0 0 1 70] AOE
  ;;[0 0 0 1 30] AOE Heal Target
  (Utilities|IsValid HealTarget
    (:Is%20Valid
      (bind (_outhit _returnvalue_2) (Collision|LineTraceByChannel _returnvalue (* _returnvalue "1.000000,1.000000,-1000.000000") "TraceTypeQuery1" false (Utilities|Array|MakeArray HealTarget) "None"))
      (if _returnvalue_2
        (bind _returnvalue_3 (Game|SpawnActorfromClass "/Game/Blueprints/Attacks/AOE/BP_AOE_Heal.BP_AOE_Heal_C" (Math|Transform|MakeTransform (.Location (Collision|BreakHitResult _outhit)) "0, 0, 0" "1.000000,1.000000,1.000000") "Undefined" "MultiplyWithRoot" 0 1.0 1e+01 false true false 0))
        (EventDispatchers|AssignOnAOEOverlapActor _returnvalue_3 (delegate Custom|OnHealTarget))
        (Default|Trigger _returnvalue_3)))))

(event Custom|OnProjectileHit
  (params (OtherActor :type Actor%20Object%20Reference) (Hit :type Hit%20Result%20Structure))
  (bind _returnvalue (Components|GetOwner))
  ;[0 0 0 1 70] Misc
  ;;[0 0 0 1 30] Magic Spell
  (Class|BPIDamageable|TakeDamage(Message) OtherActor (stale Custom|MagicSpell DamageInfo) _returnvalue)
  (Class|AISenseDamage|ReportDamageEvent 0 _returnvalue (.amount (Utilities|Struct|BreakS_DamageInfo (stale Custom|MagicSpell DamageInfo))) (Transformation|GetActorLocation (Components|GetOwner)) "0, 0, 0" "None")
  (Default|CallOnAttackEnded))

(event Custom|OnLand
  (params (Hit :type Hit%20Result%20Structure%20%28by%20ref%29))
  (bind _returnvalue (Components|GetOwner))
  (bind _ascharacter (Utilities|Casting|CastToCharacter _returnvalue))
  ;[0 0 0 1 70] Misc
  ;;[0 0 0 1 30] Jump To Attack Target
  (EventDispatchers|UnbindEventfromLandedDelegate _ascharacter (delegate Custom|OnLand))
  (Components|Movement|StopMovementImmediately (Variables|/Script/Engine.Character|GetCharacterMovement _ascharacter)))

(event Custom|LongRangedMeleeAttack
  (params (AttackInfo :type S%20Attack%20Info%20Structure) (Length :type Float%20%28single-precision%29) (Radius :type Float%20%28single-precision%29))
  (bind (_attacktarget _montage _damageinfo) (Utilities|Struct|BreakS_AttackInfo AttackInfo))
  (bind _returnvalue (Components|GetOwner))
  ;[0 0 0 1 70] Melee
  ;;[0 0 0 1 30] Long Ranged Attack
  (bind _mesh (CallFunction|AttackBase _attacktarget))
  (bind _notifyname (Animation|Montage|PlayMontage _mesh _montage)
    (:then
      (Class|BPIDamageable|SetIsInterruptable(Message) _returnvalue false))
    (:OnCompleted
      (Class|BPIEnemyAI|AttackEnd(Message) _returnvalue _attacktarget :!label _label)
      (Class|BPIDamageable|SetIsInterruptable(Message) _returnvalue true))
    (:OnInterrupted
      (goto _label))
    (:OnNotifyBegin
      (switch name _notifyname
        (:Slash
          (CallFunction|SphereTraceDamage _damageinfo Length Radius))
        (:Jump
          (CallFunction|JumptoAttackTarget _attacktarget))))))

(event Custom|LightningStrike
  (params (AttackTarget :type Actor%20Object%20Reference) (DelayBeforeStrike :type Float%20%28single-precision%29) (DamageAmount :type Float%20%28double-precision%29))
  (bind _returnvalue (Components|GetOwner))
  (bind (_aspawn _bsuccess) (Utilities|Casting|CastToPawn _returnvalue))
  ;[0 0 0 1 70] AOE
  ;;[0 0 0 1 30] AOE Lightning Strike
  (bind _returnvalue_2 (Game|SpawnActorfromClass "/Game/Blueprints/Attacks/AOE/BP_AOE_LightningStrike.BP_AOE_LightningStrike_C" (Math|Transform|MakeTransform "0, 0, 0" "0, 0, 0" "1.000000,1.000000,1.000000") "Undefined" "MultiplyWithRoot" 0 DelayBeforeStrike AttackTarget false true false (select _bsuccess _aspawn 0)))
  (EventDispatchers|AssignOnAOEOverlapActor _returnvalue_2 (delegate Custom|DamageEnemyAOE)))

(event Custom|SphereTraceDamage
  (params (DamageInfo :type S%20Damage%20Info%20Structure) (Length :type Float%20%28single-precision%29) (Radius :type Float%20%28single-precision%29))
  (bind _returnvalue (Components|GetOwner))
  (bind _returnvalue_2 (Transformation|GetActorLocation _returnvalue))
  ;[0 0 0 1 70] Misc
  ;;[0 0 0 1 30] Sphere Trace Damage
  (bind (_outhits _returnvalue_3) (Collision|MultiSphereTraceForObjects _returnvalue_2 (+ _returnvalue_2 (* (Transformation|GetActorForwardVector _returnvalue) Length)) Radius (Utilities|Array|MakeArray "ObjectTypeQuery3") false 0 "None"))
  (if _returnvalue_3
    (CallFunction|DamageAllNonTeamMembers _outhits DamageInfo)))

(event Custom|JumpToAttackTarget
  (params (AttackTarget :type Actor%20Object%20Reference))
  (bind _returnvalue (Components|GetOwner))
  (bind _ascharacter (Utilities|Casting|CastToCharacter _returnvalue))
  ;[0 0 0 1 70] Misc
  ;;[0 0 0 1 30] Jump To Attack Target
  (bind _location (CallFunction|CalculateFutureActorLocation AttackTarget 1.0))
  (bind _outlaunchvelocity (Game|SuggestProjectileVelocityCustomArc (Transformation|GetActorLocation (Components|GetOwner)) (Math|Vector|MakeVector (.x _location) (.y _location) (+ (.z _location) 1e+02)) 0.0 0.5))
  (Character|LaunchCharacter _ascharacter _outlaunchvelocity true true)
  (EventDispatchers|AssignLandedDelegate _ascharacter (delegate Custom|OnLand)))

(event Custom|BarrageAttack
  (params (AttackInfo :type S%20Attack%20Info%20Structure))
  (bind (_attacktarget _montage _damageinfo) (Utilities|Struct|BreakS_AttackInfo AttackInfo))
  (bind _returnvalue (Components|GetOwner))
  (bind _returnvalue_2 (Components|GetOwner))
  ;[0 0 0 1 70] Shooting
  ;;[0 0 0 1 30] Barrage Attack
  (bind _mesh (CallFunction|AttackBase _attacktarget))
  (bind _notifyname (Animation|Montage|PlayMontage _mesh _montage)
    (:OnCompleted
      (Class|BPIEnemyAI|AttackEnd(Message) _returnvalue :!label _label)
      (Class|BPIDamageable|SetIsInterruptable(Message) _returnvalue true))
    (:OnInterrupted
      (goto _label))
    (:OnNotifyBegin
      (switch name _notifyname
        (:Fire
          (CallFunction|MagicSpell (Math|Transform|MakeTransform (Transformation|GetSocketLocation _mesh "RightHand") (Math|Rotator|FindLookatRotation (Transformation|GetActorLocation _returnvalue_2) (+ (Transformation|GetActorLocation _returnvalue_2) (Math|Vector|MakeVector 0.0 (Math|Random|RandomFloatinRange -3e+02 3e+02) 0.0))) "1.000000,1.000000,1.000000") _attacktarget _damageinfo true)
          (Class|BPIDamageable|SetIsInterruptable(Message) _returnvalue true))))))

(event Custom|OnHealTarget
  (params (Actor :type Actor%20Object%20Reference))
  ;[0 0 0 1 70] AOE
  ;;[0 0 0 1 30] AOE Heal Target
  (if (== Actor (stale Custom|HealTarget HealTarget))
    (Class|BPIDamageable|Heal(Message) Actor 1e+01)))

(event Custom|BasicMageSpell
  (params (AttackInfo :type S%20Attack%20Info%20Structure))
  (bind (_attacktarget _montage _damageinfo) (Utilities|Struct|BreakS_AttackInfo AttackInfo))
  ;[0 0 0 1 70] Shooting
  ;;[0 0 0 1 30] Basic Magic Spell
  (bind _mesh (CallFunction|AttackBase _attacktarget))
  (bind _notifyname (Animation|Montage|PlayMontage _mesh _montage)
    (:OnCompleted
      (Class|BPIEnemyAI|AttackEnd(Message) (Components|GetOwner) _attacktarget :!label _label))
    (:OnInterrupted
      (goto _label))
    (:OnNotifyBegin
      (switch name _notifyname
        (:Fire
          (CallFunction|MagicSpell (Math|Transform|MakeTransform (Transformation|GetSocketLocation _mesh "RightHand") "0, 0, 0" "1.000000,1.000000,1.000000") _attacktarget _damageinfo false))))))

(event Custom|AOEDamage
  (params (Radius :type Float%20%28single-precision%29) (DamageInfo :type S%20Damage%20Info%20Structure))
  (bind _returnvalue (Components|GetOwner))
  ;[0 0 0 1 70] AOE
  ;;[0 0 0 1 30] AOE Damage
  (bind _returnvalue_2 (Game|SpawnActorfromClass "/Game/Blueprints/Attacks/AOE/BP_AOE_Base.BP_AOE_Base_C" (Math|Transform|MakeTransform (Transformation|GetActorLocation _returnvalue) "0, 0, 0" "1.000000,1.000000,1.000000") "Undefined" "MultiplyWithRoot" 0 true false false (.AsPawn (Utilities|Casting|CastToPawn _returnvalue))))
  (Variables|/Game/Blueprints/Attacks/AOE/BP_AOE_Base.BP_AOE_Base_C|SetRadius _returnvalue_2 Radius)
  (EventDispatchers|AssignOnAOEOverlapActor _returnvalue_2 (delegate Custom|AOEDamageActor))
  (Default|Trigger _returnvalue_2))

(event Custom|GroundSmash
  (params (AttackInfo :type S%20Attack%20Info%20Structure) (Radius :type Float%20%28single-precision%29))
  (bind (_attacktarget _montage _damageinfo) (Utilities|Struct|BreakS_AttackInfo AttackInfo))
  (bind _returnvalue (Components|GetOwner))
  ;[0 0 0 1 70] Melee
  ;;[0 0 0 1 30] Ground Smash
  (bind _mesh (CallFunction|AttackBase _attacktarget))
  (bind _notifyname (Animation|Montage|PlayMontage _mesh _montage)
    (:then
      (Class|BPIDamageable|SetIsInterruptable(Message) _returnvalue false))
    (:OnCompleted
      (Class|BPIEnemyAI|AttackEnd(Message) _returnvalue _attacktarget :!label _label)
      (Class|BPIDamageable|SetIsInterruptable(Message) _returnvalue true))
    (:OnInterrupted
      (goto _label))
    (:OnNotifyBegin
      (switch name _notifyname
        (:Smash
          (CallFunction|AOEDamage Radius _damageinfo))))))

(event Custom|CustomEvent
  (params (AttackTarget :type Actor%20Object%20Reference) (AttackInfo :type S%20Attack%20Info%20Structure))
  (bind (_attacktarget _montage _damageinfo) (Utilities|Struct|BreakS_AttackInfo AttackInfo))
  (bind _returnvalue (Components|GetOwner))
  ;[0 0 0 1 70] Misc
  ;;[0 0 0 1 30] Shoot Bullet
  (bind _mesh (CallFunction|AttackBase))
  (bind _weapon (Class|BPIDamageable|GetWeaponActor(Message) _returnvalue))
  (bind _notifyname (Animation|Montage|PlayMontage _mesh _montage)
    (:OnCompleted
      (Class|BPIEnemyAI|AttackEnd(Message) _returnvalue _attacktarget :!label _label))
    (:OnInterrupted
      (goto _label))
    (:OnNotifyBegin
      (switch name _notifyname
        (:Fire
          (CallFunction|FireBullet (Transformation|GetActorLocation _weapon) (Transformation|GetActorLocation _attacktarget) _damageinfo))))))

(event Custom|ShortRangedMelee
  (params (Attack%20Info :type S%20Attack%20Info%20Structure) (Length :type Float%20%28single-precision%29) (Radius :type Float%20%28single-precision%29))
  (bind (_attacktarget _montage _damageinfo) (Utilities|Struct|BreakS_AttackInfo Attack%20Info))
  (bind _returnvalue (Components|GetOwner))
  ;[0 0 0 1 70] Melee
  ;;[0 0 0 1 30] Short Range Melee
  (bind _mesh (CallFunction|AttackBase _attacktarget))
  (bind _notifyname (Animation|Montage|PlayMontage _mesh _montage)
    (:then
      (Class|BPIDamageable|SetIsInterruptable(Message) _returnvalue false))
    (:OnCompleted
      (Class|BPIEnemyAI|AttackEnd(Message) _returnvalue _attacktarget :!label _label)
      (Class|BPIDamageable|SetIsInterruptable(Message) _returnvalue true))
    (:OnInterrupted
      (goto _label))
    (:OnNotifyBegin
      (switch name _notifyname
        (:Slash
          (CallFunction|SphereTraceDamage _damageinfo Length Radius))))))

(fn DamageAllNonTeamMembers
  (params (Hits :type Array%20of%20Hit%20Result%20Structures) (DamageInfo :type S%20Damage%20Info%20Structure))
  (bind _teamnumber (Class|BPIDamageable|GetTeamNumber(Message) (Components|GetOwner)))
  (for _array_element Hits
    (bind _teamnumber_2 (Class|BPIDamageable|GetTeamNumber(Message) (.HitActor (Collision|BreakHitResult _array_element))))
    (if (and (not (Utilities|Array|ContainsItem (LocalVariables|GetActorsDamagedSoFar) (.HitActor (Collision|BreakHitResult _array_element)))) (!= _teamnumber_2 _teamnumber))
      (Class|BPIDamageable|TakeDamage(Message) (.HitActor (Collision|BreakHitResult _array_element)) DamageInfo (Components|GetOwner))
      (Utilities|Array|AddUnique (LocalVariables|GetActorsDamagedSoFar) (.HitActor (Collision|BreakHitResult _array_element)))))
  (return (LocalVariables|GetActorsDamagedSoFar)))

(fn DamageFirstNonTeamMember
  (params (Hits :type Array%20of%20Hit%20Result%20Structures) (Damage%20Info :type S%20Damage%20Info%20Structure))
  (bind _returnvalue (Components|GetOwner))
  (bind _teamnumber (Class|BPIDamageable|GetTeamNumber(Message) _returnvalue))
  (bind _array_element (Utilities|Array|ForEachLoopwithBreak Hits :!label _label)
    (:LoopBody
      (bind _teamnumber_2 (Class|BPIDamageable|GetTeamNumber(Message) (.HitActor (Collision|BreakHitResult _array_element))))
      (if (!= _teamnumber_2 _teamnumber)
        (Class|BPIDamageable|TakeDamage(Message) (.HitActor (Collision|BreakHitResult _array_element)) Damage%20Info _returnvalue)
        (Utilities|FlowControl|Sequence
          (:then_0
            (goto _label Break))
          (:then_1
            (return 0)))))))

(fn AttackBase
  (params (AttackTarget :type Actor%20Object%20Reference))
  (bind _returnvalue (Components|GetOwner))
  (Class|BPIEnemyAI|DefaultAttack(Message) _returnvalue AttackTarget)
  (bind _ascharacter (Utilities|Casting|CastToCharacter _returnvalue))
  (return (Variables|/Script/Engine.Character|GetMesh _ascharacter)))

(fn CalculateFutureActorLocation
  (params (Actor :type Actor%20Object%20Reference) (Time :type Float%20%28double-precision%29))
  (return (+ (Transformation|GetActorLocation Actor) (* (* (Transformation|GetVelocity Actor) "1.000000,1.000000,0.000000") Time))))
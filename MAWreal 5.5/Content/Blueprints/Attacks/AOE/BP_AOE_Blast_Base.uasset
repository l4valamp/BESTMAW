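; Base Blueprint for area-of-effect blast attacks that adds the visual and audio feedback when triggered.
; Trigger runs the parent logic, then attaches the blast particle emitter to the root and plays the blast sound at the actor's location at reduced volume.
; The actor destroys itself when the particle system finishes, or after a short delay if no effect is set.
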(event Custom|SystemFinishedEvent
  (params (PSystem :type Particle%20System%20Component%20Object%20Reference))
  (Actor|DestroyActor))

(event Custom|SpawnBlastEffects
  (bind _blasteffect (Variables|Default|GetBlastEffect)
    (:then
      (bind _returnvalue (Effects|SpawnEmitterAttached _blasteffect (Variables|Transformation|GetRootComponent) "None"))
      (EventDispatchers|AssignOnSystemFinished _returnvalue (delegate Custom|SystemFinishedEvent)))
    (:else
      (Utilities|FlowControl|Delay 1.0)
      (Actor|DestroyActor))))

(event Custom|PlayBlastSounds
  (bind _blastsound (Variables|Default|GetBlastSound)
    (:then
      (Audio|PlaySoundatLocation _blastsound (Transformation|GetActorLocation) "0, 0, 0" 0.3 1.0 0.0 0 0 0 0))
    (:else)))

(event EventBeginPlay
  (|CallParentFunction) ; This node is disabled and will not be called.\nDrag off pins to build functionality.
)

(event EventTrigger
  (|CallParentFunction)
  (CallFunction|SpawnBlastEffects)
  (CallFunction|PlayBlastSounds))

(fn ConstructionScript
  (|CallParentFunction))